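; Player ship character Blueprint that bridges the ship to the shared HUD, floating labels and end-game menu.
; BeginPlay spawns an attached player-number label, removed when the ship is destroyed, and takes the HUD from HUDManager.
; Events update this player's health, score and ammo by index, spawn colored pop-up text and show the winner menu.
; Tick eases the health bar toward current Health and sets the label text once.
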(event Custom|DestroyNumberLabel
  (Actor|DestroyActor (Variables|Default|GetPlayerPopUpNumberLabel)))

(event EventBeginPlay
  (|CallParentFunction)
  ;[1 1 1] Spawn Player number text
  (bind _returnvalue (Game|SpawnActorfromClass "/Game/Blueprints/BP_PlayerPopUpLabel.BP_PlayerPopUpLabel_C" (Transformation|GetActorTransform) "AlwaysSpawn" 0 self))
  (Class|Actor|AttachRootComponenttoActor _returnvalue self "None" "SnapToTarget" true)
  (bind _output_get (Variables|Default|SetPlayerStringForLabel "P"))
  (Variables|Default|SetPlayerPopUpNumberLabel _returnvalue)
  (bind _outactors (Actor|GetAllActorsOfClass "/Game/Blueprints/HUDManager.HUDManager_C"))
  (for _array_element _outactors
    (Variables|Default|SetHUD (Variables|/Game/Blueprints/HUDManager.HUDManager_C|GetGlobalHUD _array_element))
    (EventDispatchers|AssignOnDestroyed (delegate Custom|DestroyNumberLabel))))

(event EventActorBeginOverlap
  (params (OtherActor :type Actor%20Object%20Reference)))

(event EventTick
  (params (DeltaSeconds :type Float%20%28single-precision%29))
  (bind _hud (Variables|Default|GetHUD))
  (bind _mplayerindex (Variables|Default|GetmPlayerIndex))
  (bind _healthbararray (Variables|/Game/Blueprints/PlayerHUD.PlayerHUD_C|GetHealthBarArray _hud))
  (bind _item (Utilities|Array|Get(acopy) _healthbararray _mplayerindex))
  (Progress|SetPercent _item (Math|Interpolation|FInterpTo (Variables|/Script/UMG.ProgressBar|GetPercent _item) (stale EventSetPlayerHealth health) 0.1 0.6))
  (if (not (Variables|Default|GetAlreadySetPlayerNumber))
    ;[1 1 1] Spawn Player number text
    (Default|CustomSetText (stale EventBeginPlay _returnvalue) (Utilities|String|Append (stale EventBeginPlay _output_get) (Utilities|String|ToString(Integer) (Variables|Default|GetmPlayerIndex))))
    (Variables|Default|SetAlreadySetPlayerNumber true)))

(event EventSetPlayerScore
  (params (score :type Integer))
  (bind _output_get (Variables|Default|SetScoreTextWithoutNumber "Score: "))
  (Rendering|Components|TextRender|SetText (Utilities|Array|Get(acopy) (Variables|/Game/Blueprints/PlayerHUD.PlayerHUD_C|GetScoreArray (Variables|Default|GetHUD)) (Variables|Default|GetmPlayerIndex)) (Utilities|Text|ToText(String) (Utilities|String|Append _output_get (Utilities|String|ToString(Integer) score)))))

(event EventCreatePopUpText
  (params (s :type String) (color :type Color%20Structure))
  (bind _returnvalue (Game|SpawnActorfromClass "/Game/Blueprints/BP_PopUpText.BP_PopUpText_C" (Transformation|GetActorTransform) "Undefined" 0 self))
  (Default|CustomSetColor _returnvalue (Math|Vector|MakeVector (Math|Conversions|ToFloat(Byte) (.r color)) (Math|Conversions|ToFloat(Byte) (.g color)) (Math|Conversions|ToFloat(Byte) (.b color))) (Math|Conversions|ToFloat(Byte) (.a color)))
  (Default|CustomSetText _returnvalue s))

(event EventSetPlayerHealth
  (params (health :type Float%20%28single-precision%29))
  (if (<= health 0.0)
    (Progress|SetPercent (Utilities|Array|Get(acopy) (Variables|/Game/Blueprints/PlayerHUD.PlayerHUD_C|GetHealthBarArray (Variables|Default|GetHUD)) (Variables|Default|GetmPlayerIndex)) 0.0)))

(event EventSetPlayerVisibility
  (params (index :type Integer))
  (Widget|SetVisibility (Utilities|Array|Get(acopy) (Variables|/Game/Blueprints/PlayerHUD.PlayerHUD_C|GetHealthBarArray (Variables|Default|GetHUD)) index) "Visible"))

(event EventSetPlayerAmmo
  (params (ammo :type Integer))
  (bind _output_get (Variables|Default|SetAmmoTextWithoutNumber "Ammo: "))
  (Rendering|Components|TextRender|SetText (Utilities|Array|Get(acopy) (Variables|/Game/Blueprints/PlayerHUD.PlayerHUD_C|GetAmmoArray (Variables|Default|GetHUD)) (Variables|Default|GetmPlayerIndex)) (Utilities|Text|ToText(String) (Utilities|String|Append _output_get (Utilities|String|ToString(Integer) ammo)))))

(event EventShowEndGameMenu
  (params (playerID :type Integer))
  (bind _returnvalue (UserInterface|CreateWidget "/Game/Blueprints/EndGameMenu.EndGameMenu_C"))
  (bind _output_get (Variables|Default|SetEndGameMenu _returnvalue))
  (UserInterface|Viewport|AddtoViewport _output_get 0)
  (Default|SetWinText (Variables|Default|GetEndGameMenu) playerID))

(fn ConstructionScript)

(fn SetHUD
  (params (playerHUD :type Player%20HUD%20Object%20Reference))
  (Variables|Default|SetHUD playerHUD))