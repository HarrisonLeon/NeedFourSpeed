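; BP_PlayerPopUpLabel is a pop-up text label actor built around a TextRender component.
; On BeginPlay it shifts itself from its spawn location by OffsetX and OffsetY, keeping Z unchanged.
; CustomSetText sets the displayed text, and CustomSetColor combines the stored Color vector with a passed alpha for the render color.
; Tick is empty and an unconnected MoveComponentTo node never runs, so the label does not animate itself.
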(event EventBeginPlay
  (bind _returnvalue (Transformation|GetActorLocation))
  (Transformation|SetActorLocation (Math|Vector|MakeVector (+ (.x _returnvalue) (Math|Conversions|ToFloat(Integer) (Variables|Default|GetOffsetX))) (+ (.y _returnvalue) (Math|Conversions|ToFloat(Integer) (Variables|Default|GetOffsetY))) (.z _returnvalue)) false false))

(event Collision|EventActorBeginOverlap
  (params (OtherActor :type Actor%20Object%20Reference)))

(event EventTick
  (params (DeltaSeconds :type Float%20%28single-precision%29)))

(fn ConstructionScript)

(fn CustomSetText
  (params (text :type String))
  (Rendering|Components|TextRender|SetText (Variables|Default|GetTextRender) (Utilities|Text|ToText(String) text)))

(fn CustomSetColor
  (params (Color :type Vector) (Alpha :type Float%20%28single-precision%29))
  (Rendering|Components|TextRender|SetTextRenderColor (Variables|Default|GetTextRender) (Math|Conversions|ToColor(LinearColor) (Math|Color|MakeColor (.x Color) (.y Color) (.z Color) Alpha))))