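; Short-lived pop-up text actor that shows a TextRender string and drifts until its 0.8-second lifespan ends.
; BeginPlay picks random X and Y offsets, and Tick feeds the actor location plus those offsets into MoveComponentTo on the root, leaving Z unchanged.
; CustomSetText sets the displayed string, and CustomSetColor applies the Color vector with a supplied alpha.
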(event EventBeginPlay
  (Actor|SetLifeSpan 0.8)
  (Variables|Default|SetRandomX (Math|Random|RandomIntegerinRange 30 40))
  (Variables|Default|SetRandomY (Math|Random|RandomIntegerinRange -20 20)))

(event EventActorBeginOverlap
  (params (OtherActor :type Actor%20Object%20Reference)))

(event EventTick
  (params (DeltaSeconds :type Float%20%28single-precision%29))
  (bind _returnvalue (Transformation|GetActorLocation))
  ;[1 1 1] Moving Text
  (Components|MoveComponentTo (Variables|Default|GetDefaultSceneRoot) (Math|Vector|MakeVector (+ (.x _returnvalue) (Math|Conversions|ToFloat(Integer) (Variables|Default|GetRandomX))) (+ (.y _returnvalue) (Math|Conversions|ToFloat(Integer) (Variables|Default|GetRandomY))) (.z _returnvalue)) "0, 0, 0" false false 0.2))

(fn ConstructionScript)

(fn CustomSetText
  (params (text :type String))
  (Rendering|Components|TextRender|SetText (Variables|Default|GetTextRender) (Utilities|Text|ToText(String) text)))

(fn CustomSetColor
  (params (Color :type Vector) (Alpha :type Float%20%28single-precision%29))
  (Rendering|Components|TextRender|SetTextRenderColor (Variables|Default|GetTextRender) (Math|Conversions|ToColor(LinearColor) (Math|Color|MakeColor (.x Color) (.y Color) (.z Color) Alpha))))